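; MyMrBearGameMode is the game mode for a timed game in which the player must find the BearFriend.
; BeginPlay creates the main screen widget, caches the bear and starts a looping one-second timer.
; The timer updates the countdown and time-indexed instructions, flagging game over when the bear is found or time expires.
; Tick polls those flags to show the win or lose screen, reveal the cursor and disable player input.
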(event Custom|Timer
  (bind _bearfriend (Variables|Default|GetBearFriend))
  (bind _mainscreen (Variables|Default|GetMainScreen))
  (bind _isfound (Variables|/Game/Blueprints/BP_BearFriend.BP_BearFriend_C|GetIsFound _bearfriend))
  (if _isfound
    (bind _output_get (Variables|Default|SetDidPlayerWin _isfound))
    (Variables|Default|SetGameOver _output_get)
    (elif (>= (Variables|Default|GetTotalTime) 0.0)
      (bind _result (Math|Float|DecrementFloat (Variables|Default|GetTotalTime))
        (:%20%20
          (bind _output_get_2 (Variables|Default|SetMinText (Utilities|String|ToString(Integer) (.ReturnValue (Class|KismetMathLibrary|FMod64 _result 6e+01)))))
          (bind _output_get_3 (Variables|Default|SetSecText (Utilities|String|ToString(Integer) (Class|KismetMathLibrary|ToInt64(Float) (.Remainder (Class|KismetMathLibrary|FMod64 _result 6e+01))))))
          (Variables|/Script/UMG.TextBlock|SetText (Variables|/Game/Blueprints/WBP_MainScreen.WBP_MainScreen_C|GetTimerText _mainscreen) (Utilities|Text|ToText(String) (Utilities|String|JoinStringArray (Utilities|Array|MakeArray _output_get_2 _output_get_3) ": ")))
          (Variables|/Script/UMG.TextBlock|SetText (Variables|/Game/Blueprints/WBP_MainScreen.WBP_MainScreen_C|GetInstructionText _mainscreen) (Utilities|Text|ToText(String) (Utilities|Array|Get(acopy) (Variables|Default|GetInstructions) (Math|Float|Truncate (/ _result 3e+01)))))
          (if (<= _result 0.0)
            (Variables|Default|SetGameOver (<= _result 0.0))))))))

(event EventBeginPlay
  (bind _returnvalue (Game|GetPlayerController 0))
  (bind _returnvalue_2 (UserInterface|CreateWidget "/Game/Blueprints/WBP_MainScreen.WBP_MainScreen_C"))
  (bind _output_get (Variables|Default|SetMainScreen _returnvalue_2))
  (UserInterface|Viewport|AddtoViewport _output_get 0)
  (Variables|/Script/Engine.PlayerController|SetbShowMouseCursor _returnvalue false)
  (Input|SetInputModeGameOnly _returnvalue false)
  (bind _returnvalue_3 (Actor|GetActorOfClass "/Game/Blueprints/BP_BearFriend.BP_BearFriend_C"))
  (Variables|Default|SetBearFriend _returnvalue_3)
  (Utilities|Time|SetTimerbyEvent (delegate Custom|Timer) 1.0 true false 2.0))

(event EventTick
  (params (DeltaSeconds :type Float%20%28single-precision%29))
  (bind _returnvalue (Game|GetPlayerController 0))
  (bind _mainscreen (Variables|Default|GetMainScreen))
  (bind _didplayerwin (Variables|Default|GetDidPlayerWin))
  (if (or _didplayerwin (Variables|Default|GetGameOver))
    (Widget|SetVisibility (Variables|/Game/Blueprints/WBP_MainScreen.WBP_MainScreen_C|GetGameEndScreen _mainscreen) "Visible")
    (Variables|/Script/UMG.TextBlock|SetText (Variables|/Game/Blueprints/WBP_MainScreen.WBP_MainScreen_C|GetEndGameText _mainscreen) (Utilities|Text|ToText(String) (Utilities|Array|Get(acopy) (Variables|Default|GetConclusionTexts) (Math|Integer|SelectInt 0 1 _didplayerwin))))
    (Variables|/Script/Engine.PlayerController|SetbShowMouseCursor _returnvalue true)
    (Input|DisableInput (Game|GetPlayerCharacter 0) _returnvalue)))

(fn ConstructionScript)