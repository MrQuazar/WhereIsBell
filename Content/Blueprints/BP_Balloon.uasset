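; BP_Balloon is a Blueprint that switches its Audio component to a victory or defeat sound when the game ends.
; Each Tick it casts the game mode to MyMrBearGameMode and polls DidPlayerWin, then GameOver, so a win takes priority.
; The AudioPlayed flag limits the swap to once, and the graph only calls SetSound, with no explicit Play.
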(event EventTick
  (params (DeltaSeconds :type Float%20%28single-precision%29))
  (bind _output_get (Variables|Default|SetGameMode (Game|GetGameMode)))
  (bind _asmy_mr_bear_game_mode (Utilities|Casting|CastToMyMrBearGameMode _output_get))
  (if (and (not (Variables|Default|GetAudioPlayed)) (Variables|/Game/Blueprints/MyMrBearGameMode.MyMrBearGameMode_C|GetDidPlayerWin _asmy_mr_bear_game_mode))
    (Variables|Default|SetAudioPlayed true)
    (Audio|Components|Audio|SetSound (Variables|Default|GetAudio) "/Game/Audio/rfm-1011-victory-at-last-486385.rfm-1011-victory-at-last-486385")
    (elif (and (not (Variables|Default|GetAudioPlayed)) (Variables|/Game/Blueprints/MyMrBearGameMode.MyMrBearGameMode_C|GetGameOver _asmy_mr_bear_game_mode))
      (Variables|Default|SetAudioPlayed true)
      (Audio|Components|Audio|SetSound (Variables|Default|GetAudio) "/Game/Audio/phatphrogstudio-defeat-outros-game-sounds-collection-477823.phatphrogstudio-defeat-outros-game-sounds-collection-477823"))))

(fn ConstructionScript)