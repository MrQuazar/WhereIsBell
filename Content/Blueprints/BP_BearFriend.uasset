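; BP_BearFriend is a bear friend for the player to find, apparently in a hide-and-seek game.
; On BeginPlay it silences its Audio component in Level_Menu; in other levels it plays that audio and stops the hide-and-seek music component.
; When the player pawn hits its capsule, it sets IsFound and switches the Audio sound to children's laughter.
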(event OnComponentHit(CapsuleComponent)
  (params (HitComponent :type Primitive%20Component%20Object%20Reference) (OtherActor :type Actor%20Object%20Reference) (OtherComp :type Primitive%20Component%20Object%20Reference) (NormalImpulse :type Vector :default "0, 0, 0") (Hit :type Hit%20Result%20Structure%20%28by%20ref%29))
  (if (== OtherActor (Game|Player|GetPlayerPawn 0))
    (Variables|Default|SetIsFound true)
    (Audio|Components|Audio|SetSound (Variables|Default|GetAudio) "/Game/Audio/freesound_community-kids-laugh-45357.freesound_community-kids-laugh-45357")))

(event EventBeginPlay
  (bind _returnvalue (Game|GetCurrentLevelName true))
  (if (Utilities|Enum|Equal(Enum) _returnvalue "Level_Menu")
    (Audio|Components|Audio|Stop (Variables|Default|GetAudio))
    (else
      (Audio|Components|Audio|Play (Variables|Default|GetAudio) 0.0)
      (Audio|Components|Audio|Stop (Variables|Default|Getraspberrymusic-hide-and-seek-158103)))))

(fn ConstructionScript)